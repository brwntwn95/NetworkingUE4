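; NewGameInstance is a Game Instance Blueprint that hosts multiplayer sessions through a HOSTSESSION event.
; The event creates an advanced session with the given player limit and LAN flag, attaching session name, map and game mode as extra string settings.
; On success it opens the chosen map as a listen server, and debug prints report the button press and the success or failure result.
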(event Custom|HOST%20SESSION
  (params (Max%20Players :type Integer) (bUseLAN :type Boolean) (Session%20Name :type String) (Map%20Name :type String) (Game%20Mode :type String))
  (Development|PrintString "Pressed HOST SESSION")
  (|AdvancedSession (Utilities|Array|MakeArray (Class|AdvancedSessionsLibrary|MakeLiteralSessionPropertyString "SessionName" Session%20Name) (Class|AdvancedSessionsLibrary|MakeLiteralSessionPropertyString "MapName" Map%20Name) (Class|AdvancedSessionsLibrary|MakeLiteralSessionPropertyString "GameMode" Game%20Mode)) (Game|GetPlayerController 0) Max%20Players Max%20Players bUseLAN true false true true true false false false true
    (:OnSuccess
      (Development|PrintString "Successfully created a session")
      (Game|OpenLevel(byName) (Utilities|String|StringToName Map%20Name) false "listen"))
    (:OnFailure
      (Development|PrintString "Failed created a session"))))